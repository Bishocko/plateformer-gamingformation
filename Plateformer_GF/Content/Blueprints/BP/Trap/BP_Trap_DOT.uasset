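; BP_Trap_DOT is a damage-over-time trap that hurts a FirstPersonCharacter inside its box volume.
; Begin overlap sets an in-radius flag and starts a Delay loop that passes negated Damage to GestionVie every second and prints Vie.
; End overlap clears the flag, which is checked before each delay, so an already pending tick still lands after exit.
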(event `self.Box.OnComponentBeginOverlap`
  (params (OverlappedComponent :type "PrimitiveComponent Object Reference") (OtherActor :type "Actor Object Reference") (OtherComp :type "PrimitiveComponent Object Reference") (OtherBodyIndex :type Integer) (bFromSweep :type Boolean) (SweepResult :type "HitResult Structure (by ref)"))
  (bind _asfirst_person_character (cast `/Game/Blueprints/Character/FirstPersonCharacter` OtherActor))
  (bind _output_get (set `self.PlayerinRadius` true))
  (if _output_get :!label _label
    (`KismetSystemLibrary.Delay` 1.0)
    (`/Game/Blueprints/Character/FirstPersonCharacter.GestionVie` _asfirst_person_character (* (`self.damage`) -1))
    (`KismetSystemLibrary.PrintString` (`KismetStringLibrary.Conv_IntToString` (`/Game/Blueprints/Character/FirstPersonCharacter.vie` _asfirst_person_character)))
    (goto _label)))

(event `self.Box.OnComponentEndOverlap`
  (params (OverlappedComponent :type "PrimitiveComponent Object Reference") (OtherActor :type "Actor Object Reference") (OtherComp :type "PrimitiveComponent Object Reference") (OtherBodyIndex :type Integer))
  (cast `/Game/Blueprints/Character/FirstPersonCharacter` OtherActor)
  (set `self.PlayerinRadius` false))

(fn `UserConstructionScript`)