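; Moving platform actor that travels along an editable spline at a set speed.
; Tick advances the distance, reversing, wrapping or clamping by MovementType, then moves the platform and applies spline rotation scaled per axis to its mesh.
; Construction script assigns the model, closes the spline for one movement type and sets linear or curved points.
; Stop-overlap and endpoint delay checks run, but don't gate movement.
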(event `self.ReceiveTick`
  (params (DeltaSeconds :type "Float (single-precision)"))
  (bind _current_position (`self.Current Position`))
  (bind _movement_type (`self.Movement Type`))
  (bind _movement_type_2 (`self.Movement Type`))
  (bind _spline (`self.Spline`))
  (bind _returnvalue (* DeltaSeconds (`self.Movement Speed`)))
  (bind _returnvalue_2 (+ (`KismetMathLibrary.SelectFloat` (`self.Current Position`) (`KismetMathLibrary.SelectFloat` (- (`SplineComponent.GetSplineLength` (`self.Spline`)) _current_position) _current_position (and (> _current_position (`SplineComponent.GetSplineLength` (`self.Spline`))) (or (`|EnumEquality` _movement_type "NewEnumerator2") (`|EnumEquality` _movement_type "NewEnumerator3")))) (`|EnumEquality` (`self.Movement Type`) "NewEnumerator1")) (`KismetMathLibrary.SelectFloat` (* _returnvalue -1.0) _returnvalue (and (`|EnumEquality` (`self.Movement Type`) "NewEnumerator1") (`self.Inverse`)))))
  (if (`self.touching`)
    (`KismetSystemLibrary.Delay` (`self.Duration`))
    (set `self.touching` false))
  (`self.EndTime`
    (:`true`
      _)
    (:`false`
      (`self.StartTime`
        (:`True`
          _)
        (:`false`
          _))))
  ;[1 1 1] si infé a 0
  (if (< _current_position 0.0)
    (set `self.Inverse` false)
    (else
      ;[1 1 1] si supp a 0
      (if (> _current_position (`SplineComponent.GetSplineLength` (`self.Spline`)))
        (set `self.Inverse` true))))
  (bind _output_get (set `self.Current Position` (`KismetMathLibrary.SelectFloat` _returnvalue_2 (`KismetMathLibrary.FClamp` _returnvalue_2 0.0 (`SplineComponent.GetSplineLength` (`self.Spline`))) (or (`|EnumEquality` _movement_type_2 "NewEnumerator1") (`|EnumEquality` _movement_type_2 "NewEnumerator2") (`|EnumEquality` _movement_type_2 "NewEnumerator3")))))
  (`SceneComponent.K2_SetRelativeLocation` (`self.platform`) (`SplineComponent.GetLocationAtDistanceAlongSpline` _spline _output_get "Local") false false)
  (bind (_returnvalue_roll _returnvalue_pitch _returnvalue_yaw) (`KismetMathLibrary.BreakRotator` (`SplineComponent.GetRotationAtDistanceAlongSpline` _spline _output_get "Local")))
  (bind _output_get_2 (set `self.Return Value X (Roll)` _returnvalue_roll))
  (bind _output_get_3 (set `self.Return Value Y (Pitch)` _returnvalue_pitch))
  (bind _output_get_4 (set `self.Return Value Z (Yaw)` _returnvalue_yaw))
  (`SceneComponent.K2_SetRelativeRotation` (`self.StaticMesh`) (`KismetMathLibrary.MakeRotator` (* _output_get_2 (`self.x`)) (* _output_get_3 (`self.y`)) (* _output_get_4 (`self.z`))) false false))

(event `self.stoping.OnComponentBeginOverlap`
  (params (OverlappedComponent :type "PrimitiveComponent Object Reference") (OtherActor :type "Actor Object Reference") (OtherComp :type "PrimitiveComponent Object Reference") (OtherBodyIndex :type Integer) (bFromSweep :type Boolean) (SweepResult :type "HitResult Structure (by ref)"))
  (if (== OtherComp (`self.StaticMesh`))
    (`KismetSystemLibrary.PrintString` "entré")
    (set `self.touching` true)))

(event `self.stoping.OnComponentEndOverlap`
  (params (OverlappedComponent :type "PrimitiveComponent Object Reference") (OtherActor :type "Actor Object Reference") (OtherComp :type "PrimitiveComponent Object Reference") (OtherBodyIndex :type Integer)))

(fn `custom select float`
  (params (A :type "Float (double-precision)") (B :type "Float (double-precision)") (`is A` :type Boolean))
  (returns (value :type "Float (double-precision)"))
  (locals (valueA :type "Float (double-precision)") (ValueB :type "Float (double-precision)") (total :type "Float (double-precision)"))
  (if `is A`
    (bind _output_get (set `local.valueA` A))
    (return _output_get)
    (else
      (bind _output_get_2 (set `local.ValueB` B))
      (return _output_get_2))))

(fn `UserConstructionScript`
  (bind _returnvalue (`|EnumEquality` (`self.Spline Type`) "Curve"))
  (`StaticMeshComponent.SetStaticMesh` (`self.StaticMesh`) (`self.model`))
  (`SplineComponent.SetClosedLoop` (`self.Spline`) (`|EnumEquality` (`self.Movement Type`) "NewEnumerator2") true)
  (for _index (range (+ (`SplineComponent.GetNumberOfSplinePoints` (`self.Spline`)) 1))
    (`SplineComponent.SetSplinePointType` (`self.Spline`) _index "Linear" (`KismetMathLibrary.BooleanNAND` _returnvalue true))
    (if _returnvalue
      (for _index_2 (range (+ (`SplineComponent.GetNumberOfSplinePoints` (`self.Spline`)) 1))
        (`SplineComponent.SetTangentAtSplinePoint` (`self.Spline`) _index_2 (`SplineComponent.GetTangentAtSplinePoint` (`self.Spline`) _index_2 "Local") "Local" false)))))