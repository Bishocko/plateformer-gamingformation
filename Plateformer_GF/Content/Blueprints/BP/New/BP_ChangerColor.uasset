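; BP_ChangerColor is a pickup-style trigger that changes the first-person character's color to match its own tag.
; Its first actor tag (Red, Yellow or Green) sets the point light color in the construction script and again on BeginPlay, alongside a configurable mesh.
; When the first-person character overlaps the box, it sends that tag via ChangeColorMessage and plays a 2D chime.
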(event `self.ReceiveBeginPlay`
  (bind _pointlight (`self.PointLight`))
  (switch `name` (`|GetArrayItem` (`self.Tags`))
    (:`Red`
      (bind _output_get (set `self.ColorLight` (struct :`R` 1.0 :`A` 1.0)))
      (`LightComponent.SetLightColor` _pointlight _output_get true))
    (:`Yellow`
      (bind _output_get_2 (set `self.ColorLight` (struct :`R` 1.0 :`G` 1.0 :`A` 1.0)))
      (`LightComponent.SetLightColor` _pointlight _output_get_2 true))
    (:`Green`
      (bind _output_get_3 (set `self.ColorLight` (struct :`G` 1.0 :`A` 1.0)))
      (`LightComponent.SetLightColor` _pointlight _output_get_3 true))))

(event `self.Box.OnComponentBeginOverlap`
  (params (OverlappedComponent :type "PrimitiveComponent Object Reference") (OtherActor :type "Actor Object Reference") (OtherComp :type "PrimitiveComponent Object Reference") (OtherBodyIndex :type Integer) (bFromSweep :type Boolean) (SweepResult :type "HitResult Structure (by ref)"))
  (bind _asfirst_person_character (cast `/Game/Blueprints/Character/FirstPersonCharacter` OtherActor))
  (if (== OtherActor _asfirst_person_character)
    (message `/Game/Blueprints/BP/New/CibleInterface.ChangeColor` _asfirst_person_character (`|GetArrayItem` (`self.Tags`)))
    (`GameplayStatics.PlaySound2D` "/Game/Sounds/SFX/SFX_Chime_05B.SFX_Chime_05B" 1.0 1.0 0.0 null null)))

(fn `UserConstructionScript`
  (bind _pointlight (`self.PointLight`))
  (`StaticMeshComponent.SetStaticMesh` (`self.Color`) (`self.model`))
  (switch `name` (`|GetArrayItem` (`self.Tags`))
    (:`Red`
      (bind _output_get (set `self.ColorLight` (struct :`R` 1.0 :`A` 1.0)))
      (`LightComponent.SetLightColor` _pointlight _output_get true))
    (:`Yellow`
      (bind _output_get_2 (set `self.ColorLight` (struct :`R` 1.0 :`G` 1.0 :`A` 1.0)))
      (`LightComponent.SetLightColor` _pointlight _output_get_2 true))
    (:`Green`
      (bind _output_get_3 (set `self.ColorLight` (struct :`G` 1.0 :`A` 1.0)))
      (`LightComponent.SetLightColor` _pointlight _output_get_3 true))))